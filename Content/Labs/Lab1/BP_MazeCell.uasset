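; BP_MazeCell is a maze cell actor that builds a floor and optional edge walls in its Construction Script.
; It derives wall length and thickness from GridSize, scales the Floor, and adds static mesh walls sized through SizeToCubeScale and WallHeight.
; WestWall and SouthWall toggle their own walls, while the two far walls both depend on EastWall and are nested under SouthWall.
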(event EventBeginPlay)

(event Collision|EventActorBeginOverlap
  (params (OtherActor :type Actor%20Object%20Reference)))

(event EventTick
  (params (DeltaSeconds :type Float%20%28single-precision%29)))

(fn ConstructionScript
  (bind _gridsize (Variables|Default|GetGridSize))
  (LocalVariables|SetWallLength _gridsize)
  (LocalVariables|SetWallThickness (* _gridsize 0.1))
  (Transformation|SetRelativeScale3D (Variables|Default|GetFloor) (Utilities|SizetoCubeScale (Math|Vector|MakeVector (LocalVariables|GetWallLength) (LocalVariables|GetWallLength) (LocalVariables|GetWallThickness))))
  (if (Variables|Walls|GetWestWall)
    (AddComponent|AddStaticMeshComponent false (Math|Transform|MakeTransform (Math|Vector|MakeVector 0.0 0.0 (LocalVariables|GetWallThickness)) "0, 0, 0" (Utilities|SizetoCubeScale (Math|Vector|MakeVector (LocalVariables|GetWallLength) (LocalVariables|GetWallThickness) (Variables|Default|GetWallHeight))))))
  (if (Variables|Walls|GetSouthWall)
    (AddComponent|AddStaticMeshComponent false (Math|Transform|MakeTransform (Math|Vector|MakeVector 0.0 0.0 (LocalVariables|GetWallThickness)) "0, 0, 0" (Utilities|SizetoCubeScale (Math|Vector|MakeVector (LocalVariables|GetWallThickness) (LocalVariables|GetWallLength) (Variables|Default|GetWallHeight)))))
    (if (Variables|Walls|GetEastWall)
      (AddComponent|AddStaticMeshComponent false (Math|Transform|MakeTransform (Math|Vector|MakeVector 0.0 (- (LocalVariables|GetWallLength) (LocalVariables|GetWallThickness)) (LocalVariables|GetWallThickness)) "0, 0, 0" (Utilities|SizetoCubeScale (Math|Vector|MakeVector (LocalVariables|GetWallLength) (LocalVariables|GetWallThickness) (Variables|Default|GetWallHeight)))))
      (if (Variables|Walls|GetEastWall)
        (AddComponent|AddStaticMeshComponent false (Math|Transform|MakeTransform (Math|Vector|MakeVector (- (LocalVariables|GetWallLength) (LocalVariables|GetWallThickness)) 0.0 (LocalVariables|GetWallThickness)) "0, 0, 0" (Utilities|SizetoCubeScale (Math|Vector|MakeVector (LocalVariables|GetWallThickness) (LocalVariables|GetWallLength) (Variables|Default|GetWallHeight)))))))))